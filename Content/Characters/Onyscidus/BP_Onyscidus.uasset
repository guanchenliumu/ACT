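; BP_Onyscidus is the Onyscidus character, handling damage, hit reactions and death.
; Any damage goes to HealthComponent without poise (韧性) damage; at zero health it plays the death montage, then destroys itself.
; With poise depleted, hits from RangAttack trigger front, right, left or back montages by comparing VectorCosineAngle2D to degree ranges, so a true cosine always selects front.
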(event Custom|Event%20Take%20Any%20Damage
  (params (DamagedActor :type Actor%20Object%20Reference) (Damage :type Float%20%28single-precision%29) (DamageType :type Damage%20Type%20Object%20Reference) (InstigatedBy :type Controller%20Object%20Reference) (DamageCauser :type Actor%20Object%20Reference))
  (bind _health_component (Variables|Default|GetHealth%20Component))
  (Default|AddDamge _health_component Damage 0.0)
  (if (not (> (Variables|/Game/ThirdPersonBP/Blueprints/HealthComp.HealthComp_C|GetHealth _health_component) 0.0))
    (bind _returnvalue (Animation|PlayAnimMontage "/Game/Characters/Onyscidus/Animations/Montages/AM_Onyscidus_Death.AM_Onyscidus_Death" 1.0 "None"))
    (Utilities|FlowControl|Delay _returnvalue)
    (Actor|DestroyActor)))

(event Collision|EventHit
  (params (MyComp :type Primitive%20Component%20Object%20Reference) (Other :type Actor%20Object%20Reference) (OtherComp :type Primitive%20Component%20Object%20Reference) (bSelfMoved :type Boolean) (HitLocation :type Vector :default "0, 0, 0") (HitNormal :type Vector :default "0, 0, 0") (NormalImpulse :type Vector :default "0, 0, 0") (Hit :type Hit%20Result%20Structure%20%28by%20ref%29))
  (bind _returnvalue (Transformation|GetActorForwardVector))
  (bind _returnvalue_2 (Transformation|GetActorLocation))
  (bind _returnvalue_3 (- HitLocation _returnvalue_2))
  (bind _returnvalue_4 (Class|KismetMathLibrary|VectorCosineAngle2D _returnvalue _returnvalue_3))
  (if (not bSelfMoved)
    (if (not (> (Variables|/Game/ThirdPersonBP/Blueprints/HealthComp.HealthComp_C|Get韧性 (Variables|Default|GetHealth%20Component)) 0.0))
      (Utilities|Casting|CastToRangAttack Other)
      (if (Math|Float|InRange(Float) _returnvalue_4 -45.0 45.0 true false)
        (Animation|PlayAnimMontage "/Game/Characters/Onyscidus/Animations/Montages/AM_Onyscidus_GetHitFront.AM_Onyscidus_GetHitFront" 1.0 "None")
        (elif (Math|Float|InRange(Float) _returnvalue_4 45.0 135.0 true false)
          (Animation|PlayAnimMontage "/Game/Characters/Onyscidus/Animations/Montages/AM_Onyscidus_GetHitRight.AM_Onyscidus_GetHitRight" 1.0 "None")
          (elif (Math|Float|InRange(Float) _returnvalue_4 -135.0 -45.0 true false)
            (Animation|PlayAnimMontage "/Game/Characters/Onyscidus/Animations/Montages/AM_Onyscidus_GetHitLeft.AM_Onyscidus_GetHitLeft" 1.0 "None")
            (else
              (Animation|PlayAnimMontage "/Game/Characters/Onyscidus/Animations/Montages/AM_Onyscidus_GetHitBack.AM_Onyscidus_GetHitBack" 1.0 "None"))))))))

(event EventBeginPlay
  (EventDispatchers|BindEventtoOnTakeAnyDamage (delegate Custom|Event%20Take%20Any%20Damage)))

(event EventDestroyed
  (EventDispatchers|UnbindEventfromOnTakeAnyDamage (delegate Custom|Event%20Take%20Any%20Damage)))

(fn ConstructionScript)