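; Repax enemy character that drives its AI behavior by writing Blackboard flags.
; Perception sets CanSeePlayer for Katana, Warrior or Assassin, per-Tick distance to player 0 sets IsPursue and IsAttack, and RangAttack capsule overlap sets IsHit.
; Events apply damage to a given target or to the first Repax found at BeginPlay.
; Death, health subtraction, hit montage, health-bar billboarding and attack-facing logic are disconnected, and health-widget initialization only performs a cast.
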(event OnTargetPerceptionUpdated(AIPerception)
  (params (Actor :type Actor%20Object%20Reference) (Stimulus :type AI%20Stimulus%20Structure))
  ;[1 1 1] Ai视觉
  (Utilities|FlowControl|Sequence
    (:then_0
      (Utilities|Casting|CastToKatana Actor))
    (:then_1
      (Utilities|Casting|CastToWarrior Actor))
    (:then_2
      (Utilities|Casting|CastToAssassin Actor)))
  (AI|Components|Blackboard|SetValueasBool (AI|GetBlackboard 0) (Utilities|Name|MakeLiteralName "CanSeePlayer") (.bSuccessfullySensed (Utilities|Struct|BreakAIStimulus Stimulus))))

(event OnComponentBeginOverlap(CapsuleComponent)
  (params (OverlappedComponent :type Primitive%20Component%20Object%20Reference) (OtherActor :type Actor%20Object%20Reference) (OtherComp :type Primitive%20Component%20Object%20Reference) (OtherBodyIndex :type Integer) (bFromSweep :type Boolean) (SweepResult :type Hit%20Result%20Structure%20%28by%20ref%29))
  ;[1 1 1] 受击动画
  (Utilities|Casting|CastToRangAttack OtherActor)
  (AI|Components|Blackboard|SetValueasBool (AI|GetBlackboard 0) (Utilities|Name|MakeLiteralName "IsHit") true))

(event Custom|Initialize%20Health
  (Utilities|Casting|CastToWB_EnemyUI (UserInterface|GetWidget (Variables|Default|GetWidget))))

(event Custom|DoDamage
  (params (受击对象 :type Actor%20Object%20Reference) (伤害值 :type Float%20%28double-precision%29))
  (Game|Damage|ApplyDamage 受击对象 伤害值 0 0))

(event Custom|收到伤害
  ;[1 1 1] 敌人伤害事件（断开）
  (Development|PrintString "Hello")
  (Game|Damage|ApplyDamage (stale EventBeginPlay _returnvalue) 2.0 0 0))

(event Game|Damage|EventAnyDamage
  (params (Damage :type Float%20%28single-precision%29) (DamageType :type Damage%20Type%20Object%20Reference) (InstigatedBy :type Controller%20Object%20Reference) (DamageCauser :type Actor%20Object%20Reference))
  ;[1 1 1] 收到伤害事件后HP减少（断开）
)

(event EventBeginPlay
  ;[1 1 1] 敌人伤害事件（断开）
  (Utilities|FlowControl|Sequence
    (:then_1
      (CallFunction|InitializeHealth))
    (:then_2
      (bind _returnvalue (Actor|GetActorOfClass "BP_Enemy_Repax01_C")))))

(event EventTick
  (params (DeltaSeconds :type Float%20%28single-precision%29))
  (bind _returnvalue (AI|GetBlackboard 0))
  (bind _returnvalue_2 (AI|GetBlackboard 0))
  (bind _returnvalue_3 (Utilities|Name|MakeLiteralName "IsPursue"))
  (bind _returnvalue_4 (Transformation|GetActorLocation))
  (bind _returnvalue_5 (Game|GetPlayerCharacter 0))
  (bind _returnvalue_6 (Utilities|Name|MakeLiteralName "IsAttack"))
  (bind _returnvalue_7 (Transformation|GetActorLocation _returnvalue_5))
  (bind _returnvalue_8 (- _returnvalue_4 _returnvalue_7))
  (bind _returnvalue_9 (Math|Vector|VectorLength _returnvalue_8))
  ;[1 1 1] 判断玩家与敌人的距离
  (Utilities|FlowControl|Sequence
    (:then_0
      (if (< _returnvalue_9 1.2e+03)
        (AI|Components|Blackboard|SetValueasBool _returnvalue_2 _returnvalue_3 true)
        (else
          (AI|Components|Blackboard|SetValueasBool _returnvalue_2 _returnvalue_3 false))))
    (:then_1
      (if (< _returnvalue_9 1.8e+02)
        (AI|Components|Blackboard|SetValueasBool _returnvalue _returnvalue_6 true)
        (else
          (AI|Components|Blackboard|SetValueasBool _returnvalue _returnvalue_6 false))))))

(event Collision|EventHit
  (params (MyComp :type Primitive%20Component%20Object%20Reference) (Other :type Actor%20Object%20Reference) (OtherComp :type Primitive%20Component%20Object%20Reference) (bSelfMoved :type Boolean) (HitLocation :type Vector :default "0, 0, 0") (HitNormal :type Vector :default "0, 0, 0") (NormalImpulse :type Vector :default "0, 0, 0") (Hit :type Hit%20Result%20Structure%20%28by%20ref%29))
  ;[1 1 1] 敌人伤害事件（断开）
)

(fn ConstructionScript)

(fn 攻击朝向玩家
  (bind _as_katana (Variables|Default|GetAs%20Katana))
  (Utilities|IsValid _as_katana
    (:Is%20Valid
      (Transformation|SetActorRotation (Math|Rotator|FindLookatRotation (Transformation|GetActorLocation) (Transformation|GetActorLocation _as_katana))))))